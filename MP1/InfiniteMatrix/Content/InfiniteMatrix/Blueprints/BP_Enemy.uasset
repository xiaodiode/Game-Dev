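; BP_Enemy is an enemy actor that damages the player on contact and dies when shot.
; When its Enemy component overlaps BP_Player, it subtracts a fixed amount of health if enough remains, updates the player's health bar, shows the restart display at zero, then destroys itself.
; A hit from a BP_Bullet on the same component destroys the enemy outright.
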(event OnComponentHit(Enemy)
  (params (HitComponent :type Primitive%20Component%20Object%20Reference) (OtherActor :type Actor%20Object%20Reference) (OtherComp :type Primitive%20Component%20Object%20Reference) (NormalImpulse :type Vector :default "0, 0, 0") (Hit :type Hit%20Result%20Structure%20%28by%20ref%29))
  (Utilities|Casting|CastToBP_Bullet OtherActor)
  (Actor|DestroyActor))

(event OnComponentBeginOverlap(Enemy)
  (params (OverlappedComponent :type Primitive%20Component%20Object%20Reference) (OtherActor :type Actor%20Object%20Reference) (OtherComp :type Primitive%20Component%20Object%20Reference) (OtherBodyIndex :type Integer) (bFromSweep :type Boolean) (SweepResult :type Hit%20Result%20Structure%20%28by%20ref%29))
  (bind _asbp_player (Utilities|Casting|CastToBP_Player OtherActor))
  (if (>= (Variables|/Game/InfiniteMatrix/Blueprints/BP_Player.BP_Player_C|GetCurrentHealth _asbp_player) 1e+01)
    (bind _output_get (Variables|/Game/InfiniteMatrix/Blueprints/BP_Player.BP_Player_C|SetCurrentHealth _asbp_player (- (Variables|/Game/InfiniteMatrix/Blueprints/BP_Player.BP_Player_C|GetCurrentHealth _asbp_player) 1e+01)))
    (Default|UpdateHealthbar (Variables|/Game/InfiniteMatrix/Blueprints/BP_Player.BP_Player_C|GetHealthWidget _asbp_player) _output_get)
    (if (== _output_get 0.0)
      (Default|DisplayRestart _asbp_player)))
  (Actor|DestroyActor))

(fn ConstructionScript)